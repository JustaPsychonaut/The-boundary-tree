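; The Book actor of the intro menu, which moves between bookshelf and table, glows through custom depth, flies to the camera and opens.
; Timelines drive the shelf exit, flight and optional opening slide.
; Tick syncs the page materials' Progress parameter to the cover animation, then hides the single pages when it stops.
; Tick also sums wobble, slide and offsets from a spawned, attached FloatingComponent actor into the cover's relative location.
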(event `self.ReceiveBeginPlay`
  (`|ExecutionSequence`
    (:`then_0`
      ;[1 1 1] FloatingComponent initialization
      (bind _returnvalue (`|SpawnActorFromClass` "/Game/TheUltimateLibrary/FloatingComponent.FloatingComponent_C" (`KismetMathLibrary.MakeTransform` (0.0 0.0 0.0)) "AlwaysSpawn" "OverrideRootScale" null null))
      (bind _output_get (set `self.FloatingComponent` _returnvalue))
      (`self.K2_AttachToActor` _output_get self "None" "SnapToTarget" "SnapToTarget" "SnapToTarget" true))))

(event `MoveInsideBookshelf`
  ;[1 1 1] Relocate to table or bookshelf
  (`SceneComponent.K2_SetWorldLocationAndRotation` (`self.RootComponent`) (`self.InitLocation_InsideBookshelf`) (`self.InitRotation_InsideBookshelf`) false false))

(event `MoveOnTopOfTable`
  ;[1 1 1] Relocate to table or bookshelf
  (`SceneComponent.K2_SetWorldLocationAndRotation` (`self.RootComponent`) (`self.InitLocation_OnTopOfWorkbench`) (`self.InitRotation_OnTopOfWorkbench`) false false))

(event `StartGlowing`
  ;[1 1 1] Glow handlers
  (`PrimitiveComponent.SetRenderCustomDepth` (`self.BookCover`) true)
  (`PrimitiveComponent.SetRenderCustomDepth` (`self.PageStack_Right`) true)
  (`PrimitiveComponent.SetRenderCustomDepth` (`self.PageStack_Left`) true))

(event `StopGlowing`
  ;[1 1 1] Glow handlers
  (`PrimitiveComponent.SetRenderCustomDepth` (`self.BookCover`) false)
  (`PrimitiveComponent.SetRenderCustomDepth` (`self.PageStack_Right`) false)
  (`PrimitiveComponent.SetRenderCustomDepth` (`self.PageStack_Left`) false))

(event `GetOutsideBookshelf`
  ;[1 1 1] Animations
  (if (`self.IsInsideBookshelf`)
    (bind (_direction _factor) (`Timeline|0,5s up straight curve` :!via `PlayFromStart`)
      (:`Update`
        (`SceneComponent.K2_SetWorldLocation` (`self.Root`) (+ (`self.InitLocation_InsideBookshelf`) (* (`SceneComponent.GetForwardVector` (`self.BookCover`)) (* _factor -1.0 (`self.OutsideBookshelf_CoordOffset`)))) false false))
      (:`Finished`
        (set `self.IsInsideBookshelf` false)))))

(event `FlyToCamera`
  (bind _rootcomponent (`self.RootComponent`))
  ;[1 1 1] Animations
  (if (!= (`self.OutsideBookshelf_FinalLocation`) (0.0 0.0 0.0))
    (`/Engine/EditorBlueprintResources/StandardMacros.DoOnce` false
      (:`Completed`
        (set `self.OutsideBookshelf_InitLocation` (`SceneComponent.K2_GetComponentLocation` (`self.RootComponent`)))
        (bind (_direction _factor) (`Timeline|4s up straight curve`)
          (:`Update`
            (`SceneComponent.K2_SetWorldLocation` _rootcomponent (`KismetMathLibrary.VLerp` (`self.OutsideBookshelf_InitLocation`) (`self.OutsideBookshelf_FinalLocation`) _factor) false false)
            (`SceneComponent.K2_SetWorldRotation` _rootcomponent (`KismetMathLibrary.RLerp` (`self.InitRotation_InsideBookshelf`) (`self.InitRotation_InFrontOfCamera`) _factor true) false false)))))
    (else
      (`KismetSystemLibrary.PrintString` "ERROR. FlyToCamera final location is 0!" true true (struct :`R` 1.0 :`A` 1.0)))))

(event `self.ReceiveTick`
  (params (DeltaSeconds :type "Float (single-precision)"))
  (bind _wibblewobblefactor (`self.WibbleWobbleFactor`))
  (bind _returnvalue (* -1.0 (`self.WibbleWobbleFactor`)))
  (`|ExecutionSequence`
    (:`then_0`
      ;[1 1 1] Handling Book opening animation
      (if (`SkeletalMeshComponent.IsPlaying` (`self.BookCover`))
        (for _array_element (`|MakeArray` (`self.PageStack_Right`) (`self.PageStack_Left`) (`self.PageSingle_1`) (`self.PageSingle_2`) (`self.PageSingle_3`) (`self.PageSingle_4`) (`self.PageSingle_5`))
          (`MeshComponent.SetScalarParameterValueOnMaterials` _array_element "Progress" (/ (`SkeletalMeshComponent.GetPosition` (`self.BookCover`)) (`self.OpenAnimationTime`))))
        (elif (not (`self.OpenAnimationComplete`))
          (for _array_element_2 (`|MakeArray` (`self.PageSingle_1`) (`self.PageSingle_2`) (`self.PageSingle_3`) (`self.PageSingle_4`) (`self.PageSingle_5`))
            (`SceneComponent.SetHiddenInGame` _array_element_2 true false)
            (set `self.OpenAnimationComplete` true)))))
    (:`then_1`
      ;[1 1 1] Calculating WibbleWobble offset
      (`/Engine/EditorBlueprintResources/StandardMacros.Gate` true :!label _label
        (:`Exit`
          (set `self.WibbleWobbleFactor` (`KismetMathLibrary.FClamp` (+ (`self.WibbleWobbleFactor`) 0.01) 0.0 0.18))
          (set `self.RelativeLocation_WibbleWobble` (`KismetMathLibrary.MakeVector` (`KismetMathLibrary.RandomFloatInRange` _returnvalue _wibblewobblefactor) (`KismetMathLibrary.RandomFloatInRange` _returnvalue _wibblewobblefactor) (`KismetMathLibrary.RandomFloatInRange` _returnvalue _wibblewobblefactor))))))
    (:`then_2`
      ;[1 1 1] Calculating floating offset
      (bind _currentfloatingoffset (`/Game/TheUltimateLibrary/FloatingComponent.GetCurrentFloatingOffset` (`self.FloatingComponent`)))
      (set `self.RelativeLocation_FloatingOffset` _currentfloatingoffset))
    (:`then_3`
      ;[1 1 1] Calculating The Book's eventual relative location and updating it
      (`SceneComponent.K2_SetRelativeLocation` (`self.BookCover`) (+ (`self.RelativeLocation_WibbleWobble`) (`self.RelativeLocation_OpeningSlide`) (`self.RelativeLocation_FloatingOffset`)) false false))))

(event `StartWibbleWobble`
  ;[1 1 1] Calculating WibbleWobble offset
  (set `self.WibbleWobbleFactor` 0.0)
  (goto _label :!via `Open`))

(event `StopWibblwWobble`
  ;[1 1 1] Calculating WibbleWobble offset
  (`|ExecutionSequence`
    (:`then_0`
      (goto _label :!via `Close`))
    (:`then_1`
      (set `self.RelativeLocation_WibbleWobble` (0.0 0.0 0.0)))))

(event `Open`
  (params (WithSliding :type Boolean))
  ;[1 1 1] Animations
  (`SkeletalMeshComponent.PlayAnimation` (`self.BookCover`) "/Game/Menu_Intro/LevelElements/TheBook/Anim_TheBook.Anim_TheBook" false)
  (if WithSliding
    (`self.SlideForOpening`)))

(event `SlideForOpening`
  ;[1 1 1] Animations
  (bind (_direction _factor) (`Timeline|2s up straight curve` :!via `PlayFromStart`)
    (:`Update`
      (set `self.RelativeLocation_OpeningSlide` (`KismetMathLibrary.MakeVector` 0.0 (* _factor (`self.OpenAnimationSlidingOffset`)))))))

(fn `UserConstructionScript`)