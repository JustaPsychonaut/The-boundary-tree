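; BPArchive_TheCoreBook is an animated book actor in the intro menu, with a cover, two page stacks and five animated pages.
; Animate plays the cover animation, and Tick drives a "Progress" material parameter on pages and stacks from its normalized playback position, keeping them in step.
; When the cover stops playing, Tick hides the animated pages, guarded by a completion flag.
; SlideOut only stops the glow.
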(event `self.ReceiveBeginPlay`
  (`parent.ReceiveBeginPlay`)
  (for _array_element (`|MakeArray` (`self.PageStack_Right`) (`self.PageStack_Left`) (`self.AnimatedPage_1`) (`self.AnimatedPage_2`) (`self.AnimatedPage_3`) (`self.AnimatedPage_4`) (`self.AnimatedPage_5`))
    (`MeshComponent.SetScalarParameterValueOnMaterials` _array_element "Progress" 0.01)))

(event `Animate`
  (`SkeletalMeshComponent.PlayAnimation` (`self.Cover`) "/Game/Menu_Intro/LevelElements/TheBook/Anim_TheBook.Anim_TheBook" false)
  (`GameplayStatics.GetAllActorsOfClass` null))

(event `self.ReceiveTick`
  (params (DeltaSeconds :type "Float (single-precision)"))
  (if (`SkeletalMeshComponent.IsPlaying` (`self.Cover`))
    (for _array_element (`|MakeArray` (`self.PageStack_Right`) (`self.PageStack_Left`) (`self.AnimatedPage_1`) (`self.AnimatedPage_2`) (`self.AnimatedPage_3`) (`self.AnimatedPage_4`) (`self.AnimatedPage_5`))
      (`MeshComponent.SetScalarParameterValueOnMaterials` _array_element "Progress" (/ (`SkeletalMeshComponent.GetPosition` (`self.Cover`)) (`self.AnimationTime`))))
    (set `self.AnimationComplete` false)
    (elif (not (`self.AnimationComplete`))
      (for _array_element_2 (`|MakeArray` (`self.AnimatedPage_1`) (`self.AnimatedPage_2`) (`self.AnimatedPage_3`) (`self.AnimatedPage_4`) (`self.AnimatedPage_5`))
        (`SceneComponent.SetHiddenInGame` _array_element_2 true false)
        (set `self.AnimationComplete` true)))))

(event `self.SlideOut`
  (`self.StopGlowing`))

(fn `UserConstructionScript`
  (`parent.UserConstructionScript`))