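; Test Game Instance that saves and loads a BP_TestSave object in a named slot.
; LoadGame uses CheckGameSlot to validate the slot name and existence via error codes, then caches the loaded save in GameSave or prints the error in red.
; SaveGame creates the save object if missing, always sets its Stage to zero, writes it to the slot and prints the result.
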(event `LoadGame`
  (bind (_error_code _error_text) (`self.CheckGameSlot`))
  (if (== _error_code 0)
    (bind _returnvalue (`GameplayStatics.LoadGameFromSlot` (`self.GameSlotName`)))
    (bind _asbp_test_save (cast `/Game/Menu_Intro/Blueprints/BP_TestSave` _returnvalue))
    (set `self.GameSave` _asbp_test_save)
    (else
      (`KismetSystemLibrary.PrintString` _error_text true true (struct :`R` 1.0 :`G` 0.014735 :`A` 1.0)))))

(event `SaveGame`
  (`|ExecutionSequence`
    (:`then_0`
      (`/Engine/EditorBlueprintResources/StandardMacros.IsValid` (`self.GameSave`)
        (:`Is Not Valid`
          (bind _returnvalue (`GameplayStatics.CreateSaveGameObject` "/Game/Menu_Intro/Blueprints/BP_TestSave.BP_TestSave_C"))
          (set `self.GameSave` _returnvalue))))
    (:`then_1`
      (set `/Game/Menu_Intro/Blueprints/BP_TestSave.Stage` 0 (`self.GameSave`))
      (bind _returnvalue_2 (`GameplayStatics.SaveGameToSlot` (`self.GameSave`) (`self.GameSlotName`)))
      (if _returnvalue_2
        (`KismetSystemLibrary.PrintString` "OK!" true true (struct :`R` 0.14662 :`G` 1.0 :`A` 1.0))
        (else
          (`KismetSystemLibrary.PrintString` "ERROR! Game data can not be saved!" true true (struct :`R` 1.0 :`G` 0.014735 :`A` 1.0)))))))

(fn `CheckGameSlot`
  (returns (`Error code` :type Integer) (`Error text` :type String))
  (locals (Result :type String) (ErrorCode :type Integer))
  (`|ExecutionSequence`
    (:`then_0`
      (if (`KismetStringLibrary.NotEqual_StrStr` (`self.GameSlotName`))
        (bind _returnvalue (`GameplayStatics.DoesSaveGameExist` (`self.GameSlotName`)))
        (if _returnvalue
          (set `local.Result` "OK!")
          (set `local.ErrorCode` 0)
          (else
            (set `local.Result` "ERROR! Game slot does not exist!")
            (set `local.ErrorCode` 2)))
        (else
          (set `local.Result` "ERROR! Game slot name is not defined!")
          (set `local.ErrorCode` 1))))
    (:`then_1`
      (return (`local.ErrorCode`) (`local.Result`)))))