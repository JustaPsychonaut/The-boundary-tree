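; Intro-menu book actor that can glow via custom depth and slide out along its forward vector when animatable.
; SlideOut and SlideIn drive relative location with two timelines, and SlideIn stops the outward motion and eases back from wherever the book reached.
; The construction script applies the configurable mesh.
; Line traces for finding four neighboring books exist but are disconnected, leaving UpdateAdjacentBooks empty.
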(event `StartGlowing`
  (`PrimitiveComponent.SetRenderCustomDepth` (`self.Book`) true))

(event `StopGlowing`
  (`PrimitiveComponent.SetRenderCustomDepth` (`self.Book`) false))

(event `SlideOut`
  (if (and (`self.Animatable`) (not (`self.SlidingOut`)))
    (set `self.SlidingOut` true)
    (bind (_direction _offset) (`Timeline|0,5s up straight curve` :!via `PlayFromStart` :!label _label)
      (:`Update`
        (`SceneComponent.K2_SetRelativeLocation` (`self.Book`) (`KismetMathLibrary.VLerp` (0.0 0.0 0.0) (* (`SceneComponent.GetForwardVector` (`self.Book`)) (`self.SlideDistance`)) _offset) false false)))))

(event `UpdateAdjacentBooks`)

(event `SlideIn`
  (if (and (`self.Animatable`) (`self.SlidingOut`))
    (`|ExecutionSequence`
      (:`then_0`
        (goto _label :!via `Stop`))
      (:`then_1`
        (set `self.SlidingOut` false)
        (set `self.WhereSelfEndedUpSlidingRelativeLocation` (`SceneComponent.RelativeLocation` (`self.Book`)))
        (bind (_direction _offset) (`Timeline|0,5s up straight curve 2` :!via `PlayFromStart`)
          (:`Update`
            (`SceneComponent.K2_SetRelativeLocation` (`self.Book`) (`KismetMathLibrary.VLerp` (`self.WhereSelfEndedUpSlidingRelativeLocation`) (0.0 0.0 0.0) _offset) false false)))))))

(fn `GetMeshLocation`
  (returns (BookMeshLocation :type "Vector Structure"))
  (return (`PrimitiveComponent.GetCenterOfMass` (`self.Book`) "None")))

(fn `UserConstructionScript`
  (`StaticMeshComponent.SetStaticMesh` (`self.Book`) (`self.BookMesh`)))