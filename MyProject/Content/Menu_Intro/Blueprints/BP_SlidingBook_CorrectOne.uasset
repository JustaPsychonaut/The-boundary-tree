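; Intro-menu Blueprint for the "correct" sliding book, acting as a stand-in for a referenced book, TheBook.
; Slidein and SlideOut are empty, so these events do no sliding here.
; StartGlowing and StopGlowing forward to TheBook, and GetMeshLocation returns the center of mass of that book's Decoration1 component.
; The construction script only calls its parent.
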(event `self.SlideIn`)

(event `self.SlideOut`)

(event `self.StartGlowing`
  (`/Game/Menu_Intro/LevelElements/TheBook/BP_TheBook.StartGlowing` (`self.TheBook`)))

(event `self.StopGlowing`
  (`/Game/Menu_Intro/LevelElements/TheBook/BP_TheBook.StopGlowing` (`self.TheBook`)))

(fn `GetMeshLocation`
  (returns (BookMeshLocation :type "Vector Structure"))
  (return (`PrimitiveComponent.GetCenterOfMass` (`/Game/Menu_Intro/LevelElements/TheBook/BP_TheBook.Decoration_1` (`self.TheBook`)) "None")))

(fn `UserConstructionScript`
  (`parent.UserConstructionScript`))