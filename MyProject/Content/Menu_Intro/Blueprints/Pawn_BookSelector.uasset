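; Player pawn for the intro menu that browses books on a bookshelf and enters the next level through the correct one.
; Arrow keys move between adjacent books, with a VectorQueue feeding camera position, and the main action slides the book out.
; The correct book locks control and runs a delay-and-timeline sequence that pulls back the camera and floats the book open.
; A click then flies the camera into it, fading white before loading NextLevel.
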(event `self.ReceiveBeginPlay`
  (bind _camera (`self.Camera`))
  (bind _returnvalue (`SceneComponent.K2_GetComponentLocation` _camera))
  (bind _bookshelfcomponent (`/Game/Menu_Intro/LevelElements/BookShelf/BP_Bookshelf.BookshelfComponent` (`self.Bookshelf_Actor`)))
  (bind _returnvalue_2 (* (`SceneComponent.GetUpVector` (`/Game/Menu_Intro/LevelElements/BookShelf/BP_Bookshelf.BookshelfComponent` (`self.Bookshelf_Actor`))) (`|GetArrayItem` (`self.Bookshelf_Levels`) (`self.Bookshelf_CurrentLevel`))))
  ;[1 1 1] Initialization
  (`|ExecutionSequence`
    (:`then_0`
      (set `/Game/TheUltimateLibrary/VectorQueue.Delay` 1.0 (`self.VectorQueue`)))
    (:`then_1`
      (`/Engine/EditorBlueprintResources/StandardMacros.IsValid` (`self.Bookshelf_Actor`)
        (:`Is Valid`
          (set `self.Bookshelf_CurrentLevel` 2 :!label _label)
          (`SceneComponent.K2_SetWorldLocationAndRotation` (`self.Scene`) (+ (`SceneComponent.K2_GetComponentLocation` _bookshelfcomponent) (* (`SceneComponent.GetRightVector` _bookshelfcomponent) (`self.Bookshelf_DefaultControllerOffset_X`))) (`KismetMathLibrary.ComposeRotators` (`SceneComponent.K2_GetComponentRotation` _bookshelfcomponent) (struct :`Yaw` -90.0)) false false)
          (`SceneComponent.K2_SetRelativeLocation` (`self.Camera`) _returnvalue_2 false false)
          (`SceneComponent.K2_SetRelativeLocation` (`self.Cursor`) _returnvalue_2 false false)
          (set `self.Camera_FinalLocation` (`KismetMathLibrary.MakeVector` -24.0 0.0 (`|GetArrayItem` (`self.Bookshelf_Levels`) 2)))
          (bind (_outhit _returnvalue_3) (`KismetSystemLibrary.SphereTraceSingleForObjects` _returnvalue (+ _returnvalue (* (`SceneComponent.GetForwardVector` _camera) 100.0)) 10.0 (`|MakeArray` "ObjectTypeQuery8" :!type "EObjectTypeQuery Enum")))
          (if _returnvalue_3
            (bind _asbp_sliding_book (cast `/Game/Menu_Intro/Blueprints/BP_SlidingBook` (`.HitActor` (`GameplayStatics.BreakHitResult` _outhit))))
            (`self.ChangeBookScope` _asbp_sliding_book)
            (else
              (`KismetSystemLibrary.PrintString` "ERROR. No books found in shelf!" true true (struct :`R` 1.0 :`A` 1.0) 10.0)
              (`self.K2_DestroyActor`))))
        (:`Is Not Valid`
          (`|ExecutionSequence`
            (:`then_0`
              (bind _outactors (`GameplayStatics.GetAllActorsOfClass` "/Game/Menu_Intro/LevelElements/BookShelf/BP_Bookshelf.BP_Bookshelf_C"))
              (if (> (`KismetArrayLibrary.Array_Length` _outactors) 0)
                (set `self.Bookshelf_Actor` (`|GetArrayItem` _outactors))
                (else
                  (`KismetSystemLibrary.PrintString` "ERROR. Bookshelf doesn't exist!" true true (struct :`R` 1.0 :`A` 1.0) 10.0)
                  (`self.K2_DestroyActor`))))
            (:`then_1`
              (goto _label))))))))

(event `Key|Up`
  (params (Key :type "Key Structure"))
  (bind _topadjacentbook (`/Game/Menu_Intro/Blueprints/BP_SlidingBook.TopAdjacentBook` (`self.BookInScope`)))
  (:`Pressed`
    (if (`self.PlayerControlEnabled`)
      (`/Engine/EditorBlueprintResources/StandardMacros.IsValid` _topadjacentbook
        (:`Is Valid`
          (`self.ChangeBookScope` _topadjacentbook))))))

(event `Key|Left`
  (params (Key :type "Key Structure"))
  (bind _leftadjacentbook (`/Game/Menu_Intro/Blueprints/BP_SlidingBook.LeftAdjacentBook` (`self.BookInScope`)))
  (:`Pressed`
    (if (`self.PlayerControlEnabled`)
      (`/Engine/EditorBlueprintResources/StandardMacros.IsValid` _leftadjacentbook
        (:`Is Valid`
          (`self.ChangeBookScope` _leftadjacentbook))))))

(event `InputAction|MainAction`
  (params (Key :type "Key Structure"))
  ;[1 1 1] Book selection
  (:`Pressed`
    (if (`self.PlayerControlEnabled`)
      (`/Engine/EditorBlueprintResources/StandardMacros.IsValid` (`self.BookInScope`)
        (:`Is Valid`
          (`/Game/Menu_Intro/Blueprints/BP_SlidingBook.SlideOut` (`self.BookInScope`))
          (cast `/Game/Menu_Intro/Blueprints/BP_SlidingBook_CorrectOne` (`self.BookInScope`))
          (set `self.PlayerControlEnabled` false))))))

(event `Key|Down`
  (params (Key :type "Key Structure"))
  (bind _bottomadjacentbook (`/Game/Menu_Intro/Blueprints/BP_SlidingBook.BottomAdjacentBook` (`self.BookInScope`)))
  (:`Pressed`
    (if (`self.PlayerControlEnabled`)
      (`/Engine/EditorBlueprintResources/StandardMacros.IsValid` _bottomadjacentbook
        (:`Is Valid`
          (`self.ChangeBookScope` _bottomadjacentbook))))))

(event `Key|Right`
  (params (Key :type "Key Structure"))
  (bind _rightadjacentbook (`/Game/Menu_Intro/Blueprints/BP_SlidingBook.RightAdjacentBook` (`self.BookInScope`)))
  (:`Pressed`
    (if (`self.PlayerControlEnabled`)
      (`/Engine/EditorBlueprintResources/StandardMacros.IsValid` _rightadjacentbook
        (:`Is Valid`
          (`self.ChangeBookScope` _rightadjacentbook))))))

(event `InputAxisKey|MouseX`
  (params (AxisValue :type "Float (single-precision)"))
  ;[1 1 1] Camera control
)

(event `InputAxisKey|MouseY`
  (params (AxisValue :type "Float (single-precision)"))
  ;[1 1 1] Camera control
)

(event `ZoomOut`
  (bind (_camera_thebookpickuplocation_x _camera_thebookpickuplocation_y _camera_thebookpickuplocation_z) (`KismetMathLibrary.BreakVector` (`self.Camera_TheBookPickUpLocation`)))
  ;[1 1 1] Zoom out functions
  (set `self.Camera_TheBookPickUpLocation` (`SceneComponent.RelativeLocation` (`self.Camera`)))
  (bind (_direction _factor) (`Timeline|4s up straight curve` :!via `PlayFromStart` :!label _label_2)
    (:`Update`
      (bind (_returnvalue_x _returnvalue_y) (`KismetMathLibrary.BreakVector` (`KismetMathLibrary.VLerp` (`self.Camera_TheBookPickUpLocation`) (`self.Camera_FinalLocation`) _factor)))
      (`SceneComponent.K2_SetRelativeLocation` (`self.Camera`) (`KismetMathLibrary.MakeVector` _returnvalue_x _returnvalue_y _camera_thebookpickuplocation_z) false false))))

(event `ZoomOutFast`
  (bind (_camera_thebookpickuplocation_x _camera_thebookpickuplocation_y _camera_thebookpickuplocation_z) (`KismetMathLibrary.BreakVector` (`self.Camera_TheBookPickUpLocation`)))
  ;[1 1 1] Zoom out functions
  (`|ExecutionSequence`
    (:`then_0`
      (goto _label_2 :!via `Stop`))
    (:`then_1`
      (set `self.Camera_TheBookPickUpLocation` (`SceneComponent.RelativeLocation` (`self.Camera`)))
      (bind (_direction _factor) (`Timeline|1s up straight curve` :!via `PlayFromStart`)
        (:`Update`
          (bind (_returnvalue_x _returnvalue_y) (`KismetMathLibrary.BreakVector` (`KismetMathLibrary.VLerp` (`self.Camera_TheBookPickUpLocation`) (`self.Camera_FinalLocation`) _factor)))
          (`SceneComponent.K2_SetRelativeLocation` (`self.Camera`) (`KismetMathLibrary.MakeVector` _returnvalue_x _returnvalue_y _camera_thebookpickuplocation_z) false false))))))

(event `ZoomShift`
  ;[1 1 1] Zoom out functions
  (set `self.Camera_TheBookPickUpLocation` (`SceneComponent.RelativeLocation` (`self.Camera`)))
  (bind (_direction _factor) (`Timeline|3s up straight curve` :!via `PlayFromStart`)
    (:`Update`
      (`SceneComponent.K2_SetRelativeLocation` (`self.Camera`) (`KismetMathLibrary.VLerp` (`self.Camera_TheBookPickUpLocation`) (`self.Camera_FinalLocation`) _factor) false false))))

(event `TheBook_StartFlyingToCamera`
  (bind _camera (`self.Camera`))
  ;[1 1 1] Zoom out pattern
  (goto _label_3 :!via `Open`))

(event `TheBook_StopFlyingToCamera`
  (bind _camera (`self.Camera`))
  ;[1 1 1] Zoom out pattern
  (goto _label_3 :!via `Close`))

(event `self.ReceiveTick`
  (params (DeltaSeconds :type "Float (single-precision)"))
  (bind _camera (`self.Camera`))
  (bind _floatingcomponent (`/Game/Menu_Intro/LevelElements/TheBook/BP_TheBook.FloatingComponent` (`self.TheBook_Actor`)))
  (`|ExecutionSequence`
    (:`then_0`
      ;[1 1 1] Zoom out pattern
      (if (not (`self.PlayerControlEnabled`))
        (`|ExecutionSequence`
          (:`then_0`
            (`/Engine/EditorBlueprintResources/StandardMacros.DoOnce` false
              (:`Completed`
                (bind _asbp_sliding_book_correct_one (cast `/Game/Menu_Intro/Blueprints/BP_SlidingBook_CorrectOne` (`self.BookInScope`))
                  (:`then`
                    (`/Game/Menu_Intro/Blueprints/BP_SlidingBook.StopGlowing` _asbp_sliding_book_correct_one)
                    (bind _asbp_the_book (cast `/Game/Menu_Intro/LevelElements/TheBook/BP_TheBook` (`self.GetAttachParentActor` _asbp_sliding_book_correct_one))
                      (:`then`
                        (set `self.TheBook_Actor` _asbp_the_book)
                        (`KismetSystemLibrary.Delay` 0.3)
                        (`/Game/Menu_Intro/LevelElements/TheBook/BP_TheBook.StartWibbleWobble` (`self.TheBook_Actor`))
                        (`KismetSystemLibrary.Delay` 0.3)
                        (`self.ZoomOut`)
                        (`KismetSystemLibrary.Delay` 1.2)
                        (`/Game/Menu_Intro/LevelElements/TheBook/BP_TheBook.StopWibblwWobble` (`self.TheBook_Actor`))
                        (`/Game/Menu_Intro/LevelElements/TheBook/BP_TheBook.GetOutsideBookshelf` (`self.TheBook_Actor`))
                        (`KismetSystemLibrary.Delay` 0.1)
                        (`self.ZoomOutFast`)
                        (`KismetSystemLibrary.Delay` 1.2)
                        (`self.TheBook_StartFlyingToCamera`)
                        (set `/Game/TheUltimateLibrary/FloatingComponent.PlaneDefiningObject` self _floatingcomponent)
                        (`/Game/TheUltimateLibrary/FloatingComponent.Initialize` _floatingcomponent)
                        (`KismetSystemLibrary.Delay` 0.7)
                        (`self.ZoomShift`)
                        (`KismetSystemLibrary.Delay` 2.1)
                        (`/Game/Menu_Intro/LevelElements/TheBook/BP_TheBook.Open` (`self.TheBook_Actor`) true)
                        (`KismetSystemLibrary.Delay` 1.0)
                        (`self.TheBook_StopFlyingToCamera`)
                        (set `self.TheBookReadyToSwitchLevel` true))
                      (:`CastFailed`
                        (`KismetSystemLibrary.PrintString` "ERROR. TheBook actor is not available!" true true (struct :`R` 1.0 :`A` 1.0)))))
                  (:`CastFailed`
                    (`KismetSystemLibrary.PrintString` "ERROR. TheBook collision actor is not available!" true true (struct :`R` 1.0 :`A` 1.0)))))))
          (:`then_1`
            (`/Engine/EditorBlueprintResources/StandardMacros.Gate` true :!label _label_3
              (:`Exit`
                (`/Engine/EditorBlueprintResources/StandardMacros.IsValid` (`self.TheBook_Actor`)
                  (:`Is Valid`
                    (set `/Game/Menu_Intro/LevelElements/TheBook/BP_TheBook.OutsideBookshelf_FinalLocation` (+ (`SceneComponent.K2_GetComponentLocation` _camera) (* (`SceneComponent.GetForwardVector` _camera) 50.0)) (`self.TheBook_Actor`))
                    (`/Game/Menu_Intro/LevelElements/TheBook/BP_TheBook.FlyToCamera` (`self.TheBook_Actor`)))
                  (:`Is Not Valid`
                    (`KismetSystemLibrary.PrintString` "ERROR. TheBook actor is not available!" true true (struct :`R` 1.0 :`A` 1.0))))))))))
    (:`then_1`
      ;[1 0 0] ЗДЕСЬ БЫТЬ БАГАМ
      (if (`self.PlayerControlEnabled`)
        (bind _target (`/Game/TheUltimateLibrary/VectorQueue.GetTargetVector` (`self.VectorQueue`)))
        (`SceneComponent.K2_SetRelativeLocation` (`self.Camera`) _target false false)))))

(event `Key|H`
  (params (Key :type "Key Structure"))
  (bind _floatingcomponent (`/Game/Menu_Intro/LevelElements/TheBook/BP_TheBook.FloatingComponent` (`self.TheBook_Actor`)))
  (:`Pressed`
    (`/Engine/EditorBlueprintResources/StandardMacros.FlipFlop`
      (:`A`
        (`/Game/TheUltimateLibrary/FloatingComponent.Stop` _floatingcomponent))
      (:`B`
        (`/Game/TheUltimateLibrary/FloatingComponent.Initialize` _floatingcomponent)))))

(event `InputAxisKey|MouseWheelAxis`
  (params (AxisValue :type "Float (single-precision)"))
  (`CameraComponent.SetFieldOfView` (`self.Camera`) (`KismetMathLibrary.FClamp` (- (`CameraComponent.FieldOfView` (`self.Camera`)) AxisValue) 60.0 120.0)))

(event `Key|LeftMouseButton`
  (params (Key :type "Key Structure"))
  (bind _camera (`self.Camera`))
  (bind _camera_2 (`self.Camera`))
  (bind _rootcomponent (`Actor.RootComponent` (`self.TheBook_Actor`)))
  (bind _rootcomponent_2 (`Actor.RootComponent` (`self.TheBook_Actor`)))
  (bind _returnvalue (`SceneComponent.K2_GetComponentLocation` _rootcomponent_2))
  (bind _returnvalue_2 (+ _returnvalue (* (`SceneComponent.GetForwardVector` _rootcomponent_2) 50.0)))
  (:`Pressed`
    (if (`self.TheBookReadyToSwitchLevel`)
      (set `self.tmp_lastLocation` (`SceneComponent.K2_GetComponentLocation` _camera_2))
      (set `self.tmp_LastRotation` (`SceneComponent.K2_GetComponentRotation` _camera_2))
      (bind (_direction _factor) (`Timeline|SlowlyLookAtTheBook`)
        (:`Update`
          (`SceneComponent.K2_SetWorldLocation` (`self.Camera`) (`KismetMathLibrary.VLerp` (`self.tmp_lastLocation`) _returnvalue_2 _factor) false false)
          (`SceneComponent.K2_SetWorldRotation` (`self.Camera`) (`KismetMathLibrary.RLerp` (`self.tmp_LastRotation`) (`KismetMathLibrary.FindLookAtRotation` _returnvalue_2 _returnvalue) _factor true) false false)
          (if (> _factor 0.9)
            (`/Engine/EditorBlueprintResources/StandardMacros.DoOnce` false
              (:`Completed`
                (bind _ascontroller_menu_intro (cast `/Game/Menu_Intro/Controller_MenuIntro` (`GameplayStatics.GetPlayerController` 0)))
                (set `self.tmp_controller` _ascontroller_menu_intro)
                (bind (_direction_2 _factor_2) (`Timeline|ScreenFade`)
                  (:`Update`
                    (`/Game/Menu_Intro/Controller_MenuIntro.SetScreenColor` (`self.tmp_controller`) (make `LinearColor` 1.0 1.0 1.0 _factor_2))))))))
        (:`Finished`
          (set `self.tmp_lastLocation` (`SceneComponent.K2_GetComponentLocation` _camera))
          (set `self.tmp_LastRotation` (`SceneComponent.K2_GetComponentRotation` _camera))
          (bind (_direction_3 _factor_3) (`Timeline|RushIntoTheBook`)
            (:`Update`
              (`SceneComponent.K2_SetWorldLocation` (`self.Camera`) (`KismetMathLibrary.VLerp` (`self.tmp_lastLocation`) (+ (`SceneComponent.K2_GetComponentLocation` _rootcomponent) (* (`SceneComponent.GetForwardVector` _rootcomponent) 10.0)) _factor_3) false false))
            (:`Finished`
              (`/Game/Menu_Intro/Controller_MenuIntro.SetScreenColor` :`self` (`self.tmp_controller`))
              (`GameplayStatics.OpenLevel` (`self.NextLevel`)))))))))

(fn `BookZToShelfZ`
  (params (`Book Z` :type "Float (double-precision)"))
  (returns (`Shelf Z` :type "Float (double-precision)"))
  (locals (Level :type Integer) (MinDiff :type "Float (double-precision)" :default 100000.0))
  (set `local.Level` (`KismetArrayLibrary.Array_LastIndex` (`self.Bookshelf_Levels`)))
  (for (_array_element _array_index) (`self.Bookshelf_Levels`)
    (bind _returnvalue (`KismetMathLibrary.Abs` (- _array_element `Book Z`)))
    (if (> (`local.MinDiff`) _returnvalue)
      (set `local.MinDiff` _returnvalue)
      (set `local.Level` _array_index)))
  (return (`|GetArrayItem` (`self.Bookshelf_Levels`) (`local.Level`))))

(fn `ChangeBookScope`
  (params (NewBook :type "/Game/Menu_Intro/Blueprints/BP_SlidingBook Object Reference"))
  (locals (lNewBook :type "/Game/Menu_Intro/Blueprints/BP_SlidingBook Object Reference"))
  (set `local.lNewBook` NewBook)
  (`|ExecutionSequence`
    (:`then_0`
      (`/Engine/EditorBlueprintResources/StandardMacros.IsValid` (`self.BookInScope`)
        (:`Is Valid`
          (`/Game/Menu_Intro/Blueprints/BP_SlidingBook.SlideIn` (`self.BookInScope`))
          (`/Game/Menu_Intro/Blueprints/BP_SlidingBook.StopGlowing` (`self.BookInScope`))
          (set `self.BookInScope` null))))
    (:`then_1`
      (`/Engine/EditorBlueprintResources/StandardMacros.IsValid` (`local.lNewBook`)
        (:`Is Valid`
          (bind _output_get (set `self.BookInScope` (`local.lNewBook`)))
          (`/Game/Menu_Intro/Blueprints/BP_SlidingBook.StartGlowing` _output_get)
          (bind (_returnvalue_x _returnvalue_y _returnvalue_z) (`KismetMathLibrary.BreakVector` (- (`/Game/Menu_Intro/Blueprints/BP_SlidingBook.GetMeshLocation` _output_get) (`SceneComponent.K2_GetComponentLocation` (`Actor.RootComponent` (`self.Bookshelf_Actor`))))))
          (bind _output_get_2 (set `self.Camera_BookRelatedLocation` (`KismetMathLibrary.MakeVector` 0.0 _returnvalue_y (`self.BookZToShelfZ` _returnvalue_z))))
          (`/Game/TheUltimateLibrary/VectorQueue.Add` (`self.VectorQueue`) _output_get_2))))))

(fn `MoveCameraToBook`
  (bind (_returnvalue_x _returnvalue_y _returnvalue_z) (`KismetMathLibrary.BreakVector` (- (`/Game/Menu_Intro/Blueprints/BP_SlidingBook.GetMeshLocation` (`self.BookInScope`)) (`SceneComponent.K2_GetComponentLocation` (`Actor.RootComponent` (`self.Bookshelf_Actor`))))))
  (set `self.Camera_BookRelatedLocation` (`KismetMathLibrary.MakeVector` 0.0 _returnvalue_y (`self.BookZToShelfZ` _returnvalue_z)))
  (return))

(fn `UserConstructionScript`)